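; SaveGraphics holds saved graphics options for the scalable UMG menu.
; It exposes read-only getter functions for brightness, bloom, draw distance, presets and detail, each returning its stored variable directly.
; The frame rate limit getter returns a pair: the FrameRate toggle and its FrameRateValue.
; The graphs shown contain no setters, save or load calls, or logic that applies the settings.
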(fn GetBrightness
  (return (Variables|Default|GetBrightness)))

(fn GetBloom
  (return (Variables|Default|GetBloom)))

(fn GetDrawDistance
  (return (Variables|Default|GetDrawDistance)))

(fn GetPresets
  (return (Variables|Default|GetPresets)))

(fn GetDetail
  (return (Variables|Default|GetDetail)))

(fn GetLimitFrameRate
  (return (Variables|Default|GetFrameRate) (Variables|Default|GetFrameRateValue)))