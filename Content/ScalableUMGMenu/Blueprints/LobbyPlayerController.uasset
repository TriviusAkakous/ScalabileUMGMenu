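; Player controller for the multiplayer lobby that shows the local player's lobby widget and handles kicks from the server.
; On BeginPlay it links itself to LobbyPlayerState, registers with the GameInstance and creates the ServersLobby widget, which UpdatePlayerList refreshes.
; Kicking destroys the session, passes a kick message to the GameInstance and opens the menu map.
; SetupPlayerName loads the name from saved game settings, while the other Setup functions are false-returning stubs.
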(event Custom|UpdatePlayerList
  (bind _lobby (Variables|Default|GetLobby))
  (Utilities|IsValid _lobby
    (:Is%20Valid
      (Default|ShowPlayers _lobby))))

(event Custom|RepPlayerState
  (bind _aslobby_player_state (Utilities|Casting|CastToLobbyPlayerState (Variables|GetPlayerState))
    (:then
      (Variables|/Game/ScalableUMGMenu/Blueprints/LobbyPlayerState.LobbyPlayerState_C|SetPlayerController _aslobby_player_state self))
    (:CastFailed
      (Utilities|PrintStringAdvanced self "RepPlayerState" "Failed to cast to LobbyPlayerState"))))

(event Custom|RepGameInstance
  (Class|SetupInterface|SetupMouse(Message) (Variables|Default|GetGameInstance) false))

(event Custom|KickPlayer
  (params (MenuMap :type Name))
  (|DestroySession self
    (:OnSuccess
      (Class|SetupInterface|SetupKick(Message) (Variables|Default|GetGameInstance) true false "Kicked from server")
      (Game|OpenLevel(byName) MenuMap))
    (:OnFailure
      (Utilities|PrintStringAdvanced self "Kick" " Failed to destroy session"))))

(event EventBeginPlay
  (bind _self self)
  (bind _self_2 self)
  (CallFunction|RepPlayerState)
  (bind _output_get (Variables|Default|SetGameInstance (Game|GetGameInstance)))
  (bind _valid (Class|SetupInterface|SetupPlayerController(Message) _output_get _self_2))
  (if _valid
    _
    (else
      (Utilities|PrintStringAdvanced _self_2 "Event Graph" "Player Controller instance set failure")))
  (Input|SetInputModeGameOnly _self)
  (Variables|/Script/Engine.PlayerController|SetbShowMouseCursor _self true)
  (if (Pawn|IsLocalController)
    (if (Utilities|IsValid (Variables|Default|GetLobby))
      _
      (else
        (bind _returnvalue (UserInterface|CreateWidget "/Game/ScalableUMGMenu/Blueprints/Widgets/ServersLobby.ServersLobby_C"))
        (bind _output_get_2 (Variables|Default|SetLobby _returnvalue))
        (Widget|SetVisibility _output_get_2 "Visible")
        (UserInterface|Viewport|AddtoViewport _output_get_2 100)))
    (Class|WidgetBlueprintLibrary|SetFocustoGameViewport)))

(event EventSetupKickPlayer
  (params (Map :type Name))
  (CallFunction|KickPlayer Map))

(fn ConstructionScript)

(fn SetupPlayerName
  (bind _asscalable_umgmenu_instance (Utilities|Casting|CastToScalableUMGMenuInstance (Variables|Default|GetGameInstance))
    (:then
      (bind _output (Default|LoadPlayerName (Variables|/Game/ScalableUMGMenu/Blueprints/ScalableUMGMenuInstance.ScalableUMGMenuInstance_C|GetGameSettings _asscalable_umgmenu_instance)))
      (return _output))
    (:CastFailed
      (return "Fail"))))

(fn SetupGetMouse
  (return false))

(fn SetupMainMenu
  (params (Input :type Main%20Menu%20Object%20Reference))
  (return false))

(fn SetupPlayerController
  (params (Input :type Player%20Controller%20Object%20Reference))
  (return false))