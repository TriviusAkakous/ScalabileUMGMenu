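; Game instance for the scalable UMG menu, owning game settings, level travel and multiplayer session flow.
; Init builds a GameSettings save object that loads saved or INI settings, then applies graphics after a short delay to fix a startup draw-distance issue.
; Hosting creates a LAN Advanced Session and opens a listen-server level behind a loading screen; found sessions feed the server browser.
; Network and travel errors store their message and disconnect to the menu.
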(event Custom|EventSetPlayersName
  (params (Controller :type Player%20Controller%20Object%20Reference) (Input :type String))
  (Class|AdvancedSessionsLibrary|SetPlayerName Controller Input))

(event Custom|FindServer
  (params (SessionResultArray :type Array%20of%20Blueprint%20Session%20Result%20Structures))
  (CallFunction|DisplayServerBrowser SessionResultArray))

(event Custom|StartSingle
  (CallFunction|LoadingScreen)
  (Variables|Default|SetShowMouse false)
  (Game|OpenLevel(byName) "PlayableRoom" true "listen"))

(event Custom|HostMultiGame
  (params (ServerName :type String) (Map :type String) (PasswordBool :type Boolean) (Password :type String) (Host :type String) (PlayerController :type Player%20Controller%20Object%20Reference))
  (CallFunction|LoadingScreen PlayerController)
  (Utilities|FlowControl|Delay 2.0)
  (|AdvancedSession (Utilities|Array|MakeArray (Class|AdvancedSessionsLibrary|MakeLiteralSessionPropertyString "ServerName" ServerName) (Class|AdvancedSessionsLibrary|MakeLiteralSessionPropertyString "MapName" Map) (Class|AdvancedSessionsLibrary|MakeLiteralSessionPropertyBool "Password?" PasswordBool) (Class|AdvancedSessionsLibrary|MakeLiteralSessionPropertyString "Password" Password) (Class|AdvancedSessionsLibrary|MakeLiteralSessionPropertyString "Host" Host)) PlayerController 100 0 true true false true true false false false true
    (:OnSuccess
      (Variables|/Game/ScalableUMGMenu/Blueprints/GameSettings.GameSettings_C|SetIsConnected (Variables|ScalableUMGMenu|GetGameSettings) true)
      (Variables|Default|SetShowMouse true)
      (Game|OpenLevel(byName) "PlayableRoom" true "listen"))
    (:OnFailure
      (CallFunction|ErrorMessage "Failed to create session")
      (CallFunction|RemoveLoadingScreen))))

(event Custom|Disconnect
  (Development|PrintString "Disconnect command")
  (Game|OpenLevel(byName) (Variables|ScalableUMGMenu|Networking|GetMenuMap))
  (Utilities|FlowControl|Delay 1.0)
  (CallFunction|DestroySession))

(event Custom|SetSoundMix
  (params (InSoundMixModifier :type Sound%20Mix%20Object%20Reference) (InSoundClass :type Sound%20Class%20Object%20Reference) (Volume :type Float%20%28single-precision%29) (Pitch :type Float%20%28single-precision%29) (FadeInTime :type Float%20%28single-precision%29))
  (Audio|SetSoundMixClassOverride InSoundMixModifier InSoundClass Volume Pitch FadeInTime true))

(event Custom|DestroySession
  (bind _self self)
  (|DestroySession (Game|GetPlayerController 0)
    (:OnSuccess
      (Utilities|PrintStringAdvanced _self "Event Shutdown" "session shutdown success"))
    (:OnFailure
      (Utilities|PrintStringAdvanced _self "Event Shutdown" " Failed to destroy session"))))

(event Custom|DelayGraphics
  ;[1 1 1] Delay graphics console fixes startup draw distance issue
  (Utilities|FlowControl|Delay 0.5)
  (Default|RunGraphics (Variables|ScalableUMGMenu|GetGameSettings)))

(event EventShutdown
  (Utilities|PrintStringAdvanced self "Event ShutDown" "Do something?"))

(event EventHandleNetworkError
  (params (FailureType :type ENetworkFailure%20Enum :default "NetDriverAlreadyExists") (bIsServer :type Boolean))
  (Variables|ScalableUMGMenu|Networking|SetNetworkErrorMessage (Utilities|Text|ToText(String) (Utilities|String|EnumtoString FailureType)))
  (Variables|ScalableUMGMenu|Networking|SetNetworkErrorCheck true)
  (Variables|Default|SetShowMouse true)
  (Variables|Default|SetSwitch "NewEnumerator1")
  (CallFunction|Disconnect))

(event EventHandleTravelError
  (params (FailureType :type ETravelFailure%20Enum :default "NoLevel"))
  (Variables|ScalableUMGMenu|Networking|SetNetworkErrorMessage (Utilities|Text|ToText(String) (Utilities|String|EnumtoString FailureType)))
  (Variables|ScalableUMGMenu|Networking|SetNetworkErrorCheck true)
  (Variables|Default|SetShowMouse true)
  (Variables|Default|SetSwitch "NewEnumerator1")
  (CallFunction|Disconnect))

(event EventInit
  ;[1 1 1] Menu setup
  (bind _gamesettings (CallFunction|SetupGameSettings (Utilities|Array|MakeArray "SettingsAudio" "SettingsGame" "SettingsGraphics" "SettingsMouse")))
  (Variables|ScalableUMGMenu|SetGameSettings _gamesettings))

(event EventSetupKick
  (params (NetworkErrorCheck :type Boolean) (IsConnected :type Boolean) (NetworkErrorMessage :type Text))
  (Variables|ScalableUMGMenu|Networking|SetNetworkErrorCheck NetworkErrorCheck)
  (Variables|/Game/ScalableUMGMenu/Blueprints/GameSettings.GameSettings_C|SetIsConnected (Variables|ScalableUMGMenu|GetGameSettings) IsConnected)
  (Variables|ScalableUMGMenu|Networking|SetNetworkErrorMessage NetworkErrorMessage))

(event EventSetupMouse
  (params (Mouse :type Boolean))
  (Variables|Default|SetShowMouse Mouse)
  (CallFunction|LoadingScreen))

(event EventButtonDisconnect
  (Variables|Default|SetShowMouse true)
  (Variables|Default|SetSwitch "NewEnumerator1")
  (CallFunction|Disconnect))

(event EventOnSessionInviteAccepted
  (params (LocalPlayerNum :type Integer) (PersonInviting :type BP%20Unique%20Net%20Id%20Structure) (SessionToJoin :type Blueprint%20Session%20Result%20Structure%20%28by%20ref%29)))

(event EventOnSessionInviteReceived
  (params (LocalPlayerNum :type Integer) (PersonInviting :type BP%20Unique%20Net%20Id%20Structure) (AppId :type String) (SessionToJoin :type Blueprint%20Session%20Result%20Structure%20%28by%20ref%29)))

(event EventButtonHostDisconnect
  (Variables|Default|SetSwitch "NewEnumerator1")
  (Game|OpenLevel(byName) (Variables|ScalableUMGMenu|Networking|GetMenuMap)))

(event EventRunConsole
  (params (ConsoleCommand :type String))
  ;[1 1 1] Menu setup
  (Development|ExecuteConsoleCommand ConsoleCommand (Variables|ScalableUMGMenu|GetPlayerController)))

(fn RemoveMenu
  (bind _mainmenu (Variables|ScalableUMGMenu|Widgets|GetMainMenu))
  (Utilities|IsValid _mainmenu
    (:Is%20Valid
      (Widget|RemovefromParent _mainmenu))))

(fn LoadingScreen
  (params (OwningPlayer :type Player%20Controller%20Object%20Reference))
  (bind _returnvalue (UserInterface|CreateWidget "/Game/ScalableUMGMenu/Blueprints/Widgets/LoadingScreen.LoadingScreen_C" OwningPlayer))
  (bind _output_get (Variables|ScalableUMGMenu|Widgets|SetLoadingScreenWidget _returnvalue))
  (UserInterface|Viewport|AddtoViewport _output_get 1000)
  (return))

(fn ErrorMessage
  (params (Message :type String))
  (Development|PrintString Message))

(fn DisplayServerBrowser
  (params (SessionResultArray :type Array%20of%20Blueprint%20Session%20Result%20Structures))
  (bind _mainmenu (Variables|ScalableUMGMenu|Widgets|GetMainMenu))
  (bind _servers (Variables|/Game/ScalableUMGMenu/Blueprints/Widgets/MainMenu.MainMenu_C|GetServers _mainmenu))
  (bind _serverslist_widget (Variables|/Game/ScalableUMGMenu/Blueprints/Widgets/Servers.Servers_C|GetServersList_Widget _servers))
  (Variables|/Game/ScalableUMGMenu/Blueprints/Widgets/ServersList.ServersList_C|SetSessionResult _serverslist_widget SessionResultArray)
  (Default|ShowServers _serverslist_widget))

(fn RemoveLoadingScreen
  (bind _loadingscreenwidget (Variables|ScalableUMGMenu|Widgets|GetLoadingScreenWidget))
  (Utilities|IsValid _loadingscreenwidget
    (:Is%20Valid
      (Widget|RemovefromParent _loadingscreenwidget))
    (:Is%20Not%20Valid
      (bind _foundwidgets (Widget|GetAllWidgetsOfClass "/Game/ScalableUMGMenu/Blueprints/Widgets/LoadingScreen.LoadingScreen_C" true))
      (for _array_element _foundwidgets
        (Utilities|IsValid _array_element
          (:Is%20Valid
            (Widget|RemovefromParent _array_element)))))))

(fn CheckforSave
  (params (GameSettings :type Game%20Settings%20Object%20Reference))
  (bind _valid (Default|CheckSaveData GameSettings))
  (if _valid
    (Default|InitLoadSettings GameSettings)
    (CallFunction|DelayGraphics)
    (else
      (Default|SetupIniSettings GameSettings)
      (CallFunction|DelayGraphics)))
  (return))

(fn MakeDisconnectButton)

(fn SetupGameSettings
  (params (SaveFileName :type Array%20of%20Strings) (UserIndex :type Integer))
  (bind _returnvalue (SaveGame|CreateSaveGameObject "/Game/ScalableUMGMenu/Blueprints/GameSettings.GameSettings_C"))
  (bind _asgame_settings (Utilities|Casting|CastToGameSettings _returnvalue)
    (:then
      (Default|SetupInstance _asgame_settings self)
      (Default|InitVars _asgame_settings SaveFileName UserIndex (Game|GetPlayerController UserIndex))
      (CallFunction|CheckforSave _asgame_settings)
      (Default|LoadTableData _asgame_settings)
      (return _asgame_settings))
    (:CastFailed
      (Utilities|PrintStringAdvanced self "SetupGameSettingsInstance" "Unable to cast to GameSettings")
      (return 0))))

(fn ActionsSwitchInterface
  (params (Action :type Actions%20Enum :default "NewEnumerator0"))
  (return false))

(fn ActiveWidgetSwitchInterface
  (params (Input :type Integer))
  (return false))

(fn ButtonSetup
  (params (Parent :type User%20Widget%20Object%20Reference) (Text :type Text) (DefaultColour :type Linear%20Color%20Structure) (HoverColour :type Linear%20Color%20Structure) (ActiveColour :type Linear%20Color%20Structure) (TextColour :type Slate%20Color%20Structure) (Action :type Actions%20Enum :default "NewEnumerator0") (ChildofCanvas :type Canvas%20Panel%20Object%20Reference) (Position :type Vector%202D%20Structure) (Size :type Vector%202D%20Structure))
  (return 0))

(fn CommandSwitchInterface
  (params (CommandSwitch :type CommandSwitch%20Enum :default "NewEnumerator22"))
  (return false))

(fn HighlightWidget
  (params (Text :type String) (Commonwidgets :type CommonWidgets%20Enum :default "NewEnumerator0") (CycleArray :type Array%20of%20Strings) (Position :type Vector%202D%20Structure) (ChildofCanvas :type Canvas%20Panel%20Object%20Reference))
  (return 0))

(fn OutputFunction
  (return "" 0.0 0 "Unchecked" false))

(fn SetupGetMouse
  (return (Variables|Default|GetShowMouse)))

(fn SetupMainMenu
  (params (Input :type Main%20Menu%20Object%20Reference))
  (Variables|ScalableUMGMenu|Widgets|SetMainMenu Input)
  (return false))

(fn SetupPlayerController
  (params (Input :type Player%20Controller%20Object%20Reference))
  (bind _output_get (Variables|ScalableUMGMenu|SetPlayerController Input))
  (return (Utilities|IsValid _output_get)))