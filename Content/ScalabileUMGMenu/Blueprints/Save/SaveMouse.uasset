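; SaveMouse is a save-data Blueprint in the ScalabileUMGMenu project that holds the player's mouse settings.
; It stores axis inversion and sensitivity separately for the X and Y axes.
; Four getter functions each return one of these variables directly, with no setters or other logic in the graphs.
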(fn GetInvertMouseX
  (return (Variables|Default|GetInvertMouseX)))

(fn GetInvertMouseY
  (return (Variables|Default|GetInvertMouseY)))

(fn GetMouseXSensitivity
  (return (Variables|Default|GetMouseXSensitivity)))

(fn GetMouseYSensitivity
  (return (Variables|Default|GetMouseYSensitivity)))