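; Game instance for the scalable UMG menu that owns game settings and handles single-player, session and loading-screen flow.
; Init builds a GameSettings save object, loads saved or ini settings, and delays applying graphics to fix a startup draw distance issue.
; Advanced Sessions hosts LAN listen servers and feeds the server browser, with older find and join events retained.
; Network, travel, find and join failures store an error, destroy the session and return to the menu map.
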(event Custom|FindServer
  (params (SessionResultArray :type Array%20of%20Blueprint%20Session%20Result%20Structures))
  (CallFunction|DisplayServerBrowser SessionResultArray))

(event Custom|StartSingle
  (CallFunction|RemoveMenu)
  (CallFunction|LoadingScreen)
  (Game|OpenLevel(byName) (Variables|Default|GetMap) true "listen"))

(event Custom|JoinServer
  (params (SearchResult :type Blueprint%20Session%20Result%20Structure))
  ;[1 1 1] Old
  (CallFunction|LoadingScreen)
  (|JoinSession (Variables|Default|GetPlayerController) SearchResult
    (:OnSuccess
      (Variables|/Game/ScalabileUMGMenu/Blueprints/GameSettings.GameSettings_C|SetIsConnected (Variables|Default|GetGameSettings) true))
    (:OnFailure
      (Variables|Default|SetNetworkErrorMessage "Failed to join game session. Try again later.")
      (Variables|Default|SetNetworkErrorCheck true)
      (CallFunction|Disconnect))))

(event Custom|FindMulitGame
  (params (MaxResults :type Integer) (LAN :type Boolean) (ServerType :type EBPServerPresenceSearchType%20Enum) (Filters :type Array%20of%20Sessions%20Search%20Setting%20Structures))
  (bind _mainmenu (Variables|Default|GetMainMenu))
  (bind _servers (Variables|/Game/ScalabileUMGMenu/Blueprints/Widgets/MainMenu.MainMenu_C|GetServers _mainmenu))
  (bind _serverslist_widget (Variables|/Game/ScalabileUMGMenu/Blueprints/Widgets/Servers.Servers_C|GetServersList_Widget _servers))
  ;[1 1 1] Old
  (bind _results (|FindSessionsAdvanced (Variables|Default|GetPlayerController) MaxResults LAN ServerType Filters)
    (:then
      (Default|MakePopupThrobber _serverslist_widget)
      (Default|RemoveFormerSearchResults _serverslist_widget))
    (:OnSuccess
      (CallFunction|DisplayServerBrowser _results))
    (:OnFailure
      (Variables|Default|SetNetworkErrorMessage "Failed to find game session. Try again later.")
      (Variables|Default|SetNetworkErrorCheck true)
      (CallFunction|Disconnect))))

(event Custom|HostMultiGame
  (params (ServerName :type String) (Map :type String) (PasswordBool :type Boolean) (Password :type String) (Host :type String) (PlayerController :type Player%20Controller%20Object%20Reference))
  (CallFunction|LoadingScreen PlayerController)
  (Utilities|FlowControl|Delay 2.0)
  (|AdvancedSession (Utilities|Array|MakeArray (Class|AdvancedSessionsLibrary|MakeLiteralSessionPropertyString "ServerName" ServerName) (Class|AdvancedSessionsLibrary|MakeLiteralSessionPropertyString "MapName" Map) (Class|AdvancedSessionsLibrary|MakeLiteralSessionPropertyBool "Password?" PasswordBool) (Class|AdvancedSessionsLibrary|MakeLiteralSessionPropertyString "Password" Password) (Class|AdvancedSessionsLibrary|MakeLiteralSessionPropertyString "Host" Host)) PlayerController 100 0 true true false true true false false false true
    (:OnSuccess
      (Variables|/Game/ScalabileUMGMenu/Blueprints/GameSettings.GameSettings_C|SetIsConnected (Variables|Default|GetGameSettings) true)
      (CallFunction|RemoveMenu)
      (Game|OpenLevel(byName) (Variables|Default|GetMap) true "listen"))
    (:OnFailure
      (CallFunction|ErrorMessage "Failed to create session")
      (CallFunction|RemoveLoadingScreen))))

(event Custom|Disconnect
  (bind _playercontroller (Variables|Default|GetPlayerController))
  (|DestroySession _playercontroller
    (:then
      (Variables|/Game/ScalabileUMGMenu/Blueprints/GameSettings.GameSettings_C|SetIsConnected (Variables|Default|GetGameSettings) false))
    (:OnSuccess
      (Game|OpenLevel(byName) (Variables|Default|GetMenuMap)))
    (:OnFailure
      (Utilities|PrintStringAdvanced self "Event Shutdown" " Failed to destroy session")
      (Development|PrintString (Utilities|GetDisplayName _playercontroller)))))

(event Custom|SetSoundMix
  (params (InSoundMixModifier :type Sound%20Mix%20Object%20Reference) (InSoundClass :type Sound%20Class%20Object%20Reference) (Volume :type Float%20%28single-precision%29) (Pitch :type Float%20%28single-precision%29) (FadeInTime :type Float%20%28single-precision%29))
  (Audio|SetSoundMixClassOverride InSoundMixModifier InSoundClass Volume Pitch FadeInTime true))

(event Custom|DelayGraphics
  ;[1 1 1] Delay graphics console fixes startup draw distance issue
  (Utilities|FlowControl|Delay 0.5)
  (Default|RunGraphics (Variables|Default|GetGameSettings)))

(event EventShutdown
  (bind _playercontroller (Variables|Default|GetPlayerController))
  (|DestroySession _playercontroller
    (:then
      (Variables|/Game/ScalabileUMGMenu/Blueprints/GameSettings.GameSettings_C|SetIsConnected (Variables|Default|GetGameSettings) false))
    (:OnSuccess
      (Game|OpenLevel(byName) (Variables|Default|GetMenuMap)))
    (:OnFailure
      (Utilities|PrintStringAdvanced self "Event Shutdown" " Failed to destroy session")
      (Development|PrintString (Utilities|GetDisplayName _playercontroller)))))

(event EventHandleNetworkError
  (params (FailureType :type ENetworkFailure%20Enum :default "NetDriverAlreadyExists") (bIsServer :type Boolean))
  (Variables|Default|SetNetworkErrorMessage (Utilities|Text|ToText(String) (Utilities|String|EnumtoString FailureType)))
  (Variables|Default|SetNetworkErrorCheck true)
  (CallFunction|Disconnect))

(event EventHandleTravelError
  (params (FailureType :type ETravelFailure%20Enum :default "NoLevel"))
  (Variables|Default|SetNetworkErrorMessage (Utilities|Text|ToText(String) (Utilities|String|EnumtoString FailureType)))
  (Variables|Default|SetNetworkErrorCheck true)
  (CallFunction|Disconnect))

(event EventInit
  ;[1 1 1] Menu setup
  (bind _gamesettings (CallFunction|SetupGameSettings (Utilities|Array|MakeArray "SettingsAudio" "SettingsGame" "SettingsGraphics" "SettingsMouse")))
  (Variables|Default|SetGameSettings _gamesettings))

(event EventOnSessionInviteAccepted
  (params (LocalPlayerNum :type Integer) (PersonInviting :type BP%20Unique%20Net%20Id%20Structure) (SessionToJoin :type Blueprint%20Session%20Result%20Structure%20%28by%20ref%29)))

(event EventOnSessionInviteReceived
  (params (LocalPlayerNum :type Integer) (PersonInviting :type BP%20Unique%20Net%20Id%20Structure) (AppId :type String) (SessionToJoin :type Blueprint%20Session%20Result%20Structure%20%28by%20ref%29)))

(event EventRunConsole
  (params (ConsoleCommand :type String))
  ;[1 1 1] Menu setup
  (Development|ExecuteConsoleCommand ConsoleCommand (Variables|Default|GetPlayerController)))

(fn RemoveMenu
  (bind _mainmenu (Variables|Default|GetMainMenu))
  (Utilities|IsValid _mainmenu
    (:Is%20Valid
      (Widget|RemovefromParent _mainmenu))))

(fn LoadingScreen
  (params (OwningPlayer :type Player%20Controller%20Object%20Reference))
  (bind _returnvalue (UserInterface|CreateWidget "/Game/ScalabileUMGMenu/Blueprints/Widgets/LoadingScreen.LoadingScreen_C" OwningPlayer))
  (bind _output_get (Variables|Default|SetLoadingScreenWidget _returnvalue))
  (UserInterface|Viewport|AddtoViewport _output_get 0))

(fn ErrorMessage
  (params (Message :type String))
  (Development|PrintString Message))

(fn DisplayServerBrowser
  (params (SessionResultArray :type Array%20of%20Blueprint%20Session%20Result%20Structures))
  (bind _mainmenu (Variables|Default|GetMainMenu))
  (bind _servers (Variables|/Game/ScalabileUMGMenu/Blueprints/Widgets/MainMenu.MainMenu_C|GetServers _mainmenu))
  (bind _serverslist_widget (Variables|/Game/ScalabileUMGMenu/Blueprints/Widgets/Servers.Servers_C|GetServersList_Widget _servers))
  (Variables|/Game/ScalabileUMGMenu/Blueprints/Widgets/ServersList.ServersList_C|SetSessionResult _serverslist_widget SessionResultArray)
  (Default|ShowServers _serverslist_widget))

(fn RemoveLoadingScreen
  (bind _loadingscreenwidget (Variables|Default|GetLoadingScreenWidget))
  (Utilities|IsValid _loadingscreenwidget
    (:Is%20Valid
      (Widget|RemovefromParent _loadingscreenwidget))
    (:Is%20Not%20Valid
      (bind _foundwidgets (Widget|GetAllWidgetsOfClass "/Game/ScalabileUMGMenu/Blueprints/Widgets/LoadingScreen.LoadingScreen_C" true))
      (for _array_element _foundwidgets
        (Utilities|IsValid _array_element
          (:Is%20Valid
            (Widget|RemovefromParent _array_element)))))))

(fn LoadGameSettings)

(fn CheckforSave
  (params (GameSettings :type Game%20Settings%20Object%20Reference))
  (bind _valid (Default|CheckSaveData GameSettings))
  (if _valid
    (Default|InitLoadSettings GameSettings)
    (CallFunction|DelayGraphics)
    (else
      (Default|SetupIniSettings GameSettings)
      (CallFunction|DelayGraphics)))
  (return))

(fn MakeDisconnectButton)

(fn SetupGameSettings
  (params (SaveFileName :type Array%20of%20Strings) (UserIndex :type Integer))
  (bind _returnvalue (SaveGame|CreateSaveGameObject "/Game/ScalabileUMGMenu/Blueprints/GameSettings.GameSettings_C"))
  (bind _asgame_settings (Utilities|Casting|CastToGameSettings _returnvalue)
    (:then
      (Default|SetupInstance _asgame_settings self)
      (Default|InitVars _asgame_settings SaveFileName UserIndex)
      (CallFunction|CheckforSave _asgame_settings)
      (Default|LoadTableData _asgame_settings)
      (return _asgame_settings))
    (:CastFailed
      (Utilities|PrintStringAdvanced self "SetupGameSettingsInstance" "Unable to cast to GameSettings")
      (return 0))))

(fn OutputFunction
  (return "" 0.0 0 "Unchecked" false))