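; SaveAudio holds the audio settings for the ScalableUMGMenu options, judging by its name and Save folder.
; It stores volumes for master, SFX, UI, music and VOIP, plus voice chat options for microphone, push-to-talk, autotalk sensitivity and boost.
; Each value is exposed through a plain getter function, with no setters, events or save and load logic in its graphs.
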(fn GetMasterVolume
  (return (Variables|Default|GetMasterVolume)))

(fn GetSFXVolume
  (return (Variables|Default|GetSFXVolume)))

(fn GetUIVolume
  (return (Variables|Default|GetUIVolume)))

(fn GetMusicVolume
  (return (Variables|Default|GetMusicVolume)))

(fn GetVOIPVolume
  (return (Variables|Default|GetVOIPVolume)))

(fn GetMicrophoneEnabled
  (return (Variables|Default|GetMicrophoneEnabled)))

(fn GetAutotalkSensitivity
  (return (Variables|Default|GetAutotalkSensitivity)))

(fn GetMicrophoneVolumeBoost
  (return (Variables|Default|GetMicrophoneVolumeBoost)))

(fn GetPushtoTalkEnabled
  (return (Variables|Default|GetPushToTalkEnabled)))