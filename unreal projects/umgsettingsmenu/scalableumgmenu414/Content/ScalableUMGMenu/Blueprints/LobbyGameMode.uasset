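; Lobby game mode that tracks players joining and leaving a lobby and keeps their player lists up to date.
; On login and logout it edits a controller array and a parallel array of player stats structs, created with an empty name.
; After a one-second delay for replication, it tells every LobbyPlayerController to update its player list.
; Struct removal matches on controller plus empty name, logging a message on failure.
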(event EventOnLogout
  (params (ExitingController :type Controller%20Object%20Reference))
  (Utilities|Array|RemoveItem (Variables|Default|GetPlayerList) ExitingController)
  (CallFunction|RemovePlayerList ExitingController)
  ;[1 1 1] Give the server time to replicate server list
  (Utilities|FlowControl|Delay 1.0)
  (CallFunction|UpdatePlayerList))

(event EventPostLogin
  (params (NewPlayer :type Player%20Controller%20Object%20Reference))
  (Utilities|Array|Add (Variables|Default|GetPlayerList) NewPlayer)
  (CallFunction|SetupPlayerList NewPlayer)
  ;[1 1 1] Give the server time to replicate server list
  (Utilities|FlowControl|Delay 1.0)
  (CallFunction|UpdatePlayerList))

(fn ConstructionScript)

(fn UpdatePlayerList
  (for _array_element (Variables|Default|GetPlayerList)
    (bind _aslobby_player_controller (Utilities|Casting|CastToLobbyPlayerController _array_element)
      (:then
        (Default|UpdatePlayerList _aslobby_player_controller))
      (:CastFailed
        (Utilities|PrintStringAdvanced self "UpdatePlayerList" " Failed to cast to LobbyPlayerController")))))

(fn SetupPlayerList
  (params (Controller :type Controller%20Object%20Reference))
  (Utilities|Array|Add (Variables|Default|GetPlayerListStruct) (Utilities|Struct|MakePlayerStatsStruct "" Controller))
  (return))

(fn RemovePlayerList
  (params (Controller :type Controller%20Object%20Reference))
  (bind _returnvalue (Utilities|Array|RemoveItem (Variables|Default|GetPlayerListStruct) (Utilities|Struct|MakePlayerStatsStruct "" Controller)))
  (if _returnvalue
    _
    (else
      (Utilities|PrintStringAdvanced self "Remove Player List" "Failed to remove player")))
  (return))